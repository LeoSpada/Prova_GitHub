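; BP_Blocco_Sollevabile is a liftable block that serves as a concrete block, cone, battery or light bulb.
; The construction script applies the chosen mesh, enabling damage for the cone, electricity for the battery and the point light for the bulb.
; PickUp destroys the original actor a tick later.
; Tick fakes gravity, tracing downward with persistent debug lines and lowering the block at constant speed while above the impact point.
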(event EventTick
  (params (DeltaSeconds :type Float%20%28single-precision%29))
  (bind _returnvalue (Transformation|GetActorLocation))
  (bind _returnvalue_2 (Transformation|GetActorLocation))
  ;[0.15 0.15 0.15 0.5] Falling Funtion
  (bind _outhit (Collision|LineTraceByChannel _returnvalue (- _returnvalue "0.000000,0.000000,1000.000000") "TraceTypeQuery2" false 0 "Persistent"))
  (if (> (.z _returnvalue_2) (.z (.ImpactPoint (Collision|BreakHitResult _outhit))))
    (Transformation|SetActorLocation (Math|Vector|MakeVector (.x _returnvalue_2) (.y _returnvalue_2) (- (.z _returnvalue_2) (* 8e+02 DeltaSeconds))) false false)))

(event EventPickUp
  ;[0.15 0.15 0.15 0.5] Quando il blocco viene raccolto, distruggi il blocco che si trovava nella posizione originale
  (Development|PrintString "Block Picked")
  (Utilities|FlowControl|DelayUntilNextTick)
  (Actor|DestroyActor))

(fn ConstructionScript
  (bind _mesh (Variables|Default|GetMesh))
  ;[0.15 0.15 0.15 0.5] Funzione che gestisce la logica di tutti i blocchi (Blocco di cemento, Cono, Batteria e Lampadina)
  (Components|StaticMesh|SetStaticMesh (Variables|Default|GetBlocco_di_cemento) _mesh)
  (if (== "/Game/Modelli_3D/MODELLI_3D_Oggetti/Cono/Cono.Cono" _mesh)
    (Variables|Default|SetCanDMG true)
    (elif (== "/Game/Modelli_3D/MODELLI_3D_Oggetti/Batteria/Batteria_v2.Batteria_v2" _mesh)
      (Variables|Default|SetElectricity true)
      (elif (== _mesh "/Game/Modelli_3D/MODELLI_3D_Oggetti/Lampadina/Lampadina1.Lampadina1")
        (Rendering|SetVisibility (Variables|Default|GetPointLight) true false)))))