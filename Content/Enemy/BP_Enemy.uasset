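; BP_Enemy is a patrolling enemy that the player can destroy from above, with movement suited to a side-scrolling plane.
; Patrol re-calls itself after each successful AI MoveTo and short delay, cycling an index through two patrol points.
; A box overlap destroys the enemy when it meets BP_Player's Box with the player sufficiently higher.
; A movement-updated handler keeps only X and Z to stabilize Y, but is bound only within itself.
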(event OnComponentBeginOverlap(Box)
  (params (OverlappedComponent :type Primitive%20Component%20Object%20Reference) (OtherActor :type Actor%20Object%20Reference) (OtherComp :type Primitive%20Component%20Object%20Reference) (OtherBodyIndex :type Integer) (bFromSweep :type Boolean) (SweepResult :type Hit%20Result%20Structure%20%28by%20ref%29))
  (bind _asbp_player (Utilities|Casting|CastToBP_Player OtherActor))
  (if (and (== (Variables|/Game/Player/BP_Player.BP_Player_C|GetBox _asbp_player) OtherComp) (> (- (.z (Transformation|GetActorLocation _asbp_player)) (.z (Transformation|GetActorLocation))) 2.1e+02))
    (Actor|DestroyActor)))

(event Custom|OnCharacterMovementUpdated_Event
  (params (DeltaSeconds :type Float%20%28single-precision%29) (OldLocation :type Vector) (OldVelocity :type Vector))
  (bind _returnvalue (Transformation|GetActorLocation))
  ;[0.15 0.15 0.15 0.5] Help Stabilize Y Location
  (EventDispatchers|BindEventtoOnCharacterMovementUpdated (delegate Custom|OnCharacterMovementUpdated_Event))
  (Transformation|SetActorLocation (Math|Vector|MakeVector (.x _returnvalue) 0.0 (.z _returnvalue)) false false))

(event Custom|Patrol
  ;[0.15 0.15 0.15 0.5] AI
  (Variables|/Script/Engine.CharacterMovementComponent|SetMaxWalkSpeed (Variables|Character|GetCharacterMovement) 3e+02)
  (AI|AIMoveTo self (Utilities|Array|Get(acopy) (Variables|Default|GetPatrolPoints) (Variables|Default|GetPoints)) 0 5.0 false
    (:OnSuccess
      (Utilities|FlowControl|Delay 0.5)
      (CallFunction|Patrol)
      (Math|Integer|IncrementInt (Variables|Default|GetPoints)
        (:%20%20
          (if (== (Variables|Default|GetPoints) 2)
            (Variables|Default|SetPoints 0)))))))

(event EventBeginPlay
  ;[0.15 0.15 0.15 0.5] AI
  (CallFunction|Patrol))

(fn ConstructionScript)