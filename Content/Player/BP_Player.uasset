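; Player pawn for a side-scrolling game: it moves left and right, flips its mesh to face travel, jumps, and tracks health on a UI_Player widget.
; E picks up an overlapped BP_Blocco_Sollevabile through PU_Interface, shows its mesh as carried, and respawns it ahead when the box check is clear.
; Cone blocks hurt once per capsule overlap, gated by CanDMG.
; Esc or Z toggles the pause menu (commented as not working).
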(event OnComponentBeginOverlap(CapsuleComponent)
  (params (OverlappedComponent :type Primitive%20Component%20Object%20Reference) (OtherActor :type Actor%20Object%20Reference) (OtherComp :type Primitive%20Component%20Object%20Reference) (OtherBodyIndex :type Integer) (bFromSweep :type Boolean) (SweepResult :type Hit%20Result%20Structure%20%28by%20ref%29))
  ;[0.15 0.15 0.15 0.5] Danno Solo da Cono
  (bind _asbp_blocco_sollevabile (Utilities|Casting|CastToBP_Blocco_Sollevabile OtherActor))
  (if (and (== (Variables|/Game/Blocchi/BP_Blocco_Sollevabile.BP_Blocco_Sollevabile_C|GetDMG_Trigger _asbp_blocco_sollevabile) OtherComp) (and (== (Variables|/Game/Blocchi/BP_Blocco_Sollevabile.BP_Blocco_Sollevabile_C|GetMesh _asbp_blocco_sollevabile) "/Game/Modelli_3D/MODELLI_3D_Oggetti/Cono/Cono.Cono") (Variables|/Game/Blocchi/BP_Blocco_Sollevabile.BP_Blocco_Sollevabile_C|GetCanDMG _asbp_blocco_sollevabile)))
    (Utilities|FlowControl|DelayUntilNextTick)
    (bind _output_get (Variables|Default|Setcurrent_health (- (Variables|Default|Getcurrent_health) 1.0)))
    (Default|UIUpdateHealth (Variables|Default|GetUI_main) _output_get (Variables|Default|Getmax_health))
    (Variables|/Game/Blocchi/BP_Blocco_Sollevabile.BP_Blocco_Sollevabile_C|SetCanDMG _asbp_blocco_sollevabile false)))

(event OnComponentEndOverlap(CapsuleComponent)
  (params (OverlappedComponent :type Primitive%20Component%20Object%20Reference) (OtherActor :type Actor%20Object%20Reference) (OtherComp :type Primitive%20Component%20Object%20Reference) (OtherBodyIndex :type Integer))
  ;[0.15 0.15 0.15 0.5] Danno Solo da Cono
  (bind _asbp_blocco_sollevabile (Utilities|Casting|CastToBP_Blocco_Sollevabile OtherActor))
  (Variables|/Game/Blocchi/BP_Blocco_Sollevabile.BP_Blocco_Sollevabile_C|SetCanDMG _asbp_blocco_sollevabile true))

(event Input|EnhancedActionEvents|EnhancedInputActionACT_Pause_Menu
  (params (ActionValue :type Boolean) (ElapsedSeconds :type Float%20%28double-precision%29) (TriggeredSeconds :type Float%20%28double-precision%29) (InputAction :type Input%20Action%20Object%20Reference :default "/Game/Player/Azioni/ACT_Pause_Menu.ACT_Pause_Menu"))
  (bind _returnvalue (Game|GetPlayerController 0))
  ;[0.15 0.15 0.15 0.5] (MENU DI PAUSA) Quando premo "Esc", se il menù di pausa è chiuso, lo apri; ALTRIMENTI, se il menù di pausa è aperto, lo chiudi
  (if (not (Variables|Default|Getmenu_pausa_aperto?))
    (Variables|Default|Setmenu_pausa_aperto? true)
    (bind _returnvalue_2 (UserInterface|CreateWidget "/Game/Interfaccia_Grafica/UI_Pause_Menu.UI_Pause_Menu_C" _returnvalue))
    (bind _output_get (Variables|Default|Setui_menu_pausa _returnvalue_2))
    (UserInterface|Viewport|AddtoViewport _output_get 0)
    (Input|SetInputModeGameandUI _returnvalue (Variables|Default|Getui_menu_pausa) "DoNotLock" true false)
    (Variables|/Script/Engine.PlayerController|SetbShowMouseCursor (Game|GetPlayerController 0) true)
    (Game|SetGamePaused true)
    (else
      (Variables|Default|Setmenu_pausa_aperto? false)
      (Widget|RemovefromParent (Variables|Default|Getui_menu_pausa))
      (Game|SetGamePaused false)
      (Input|SetInputModeGameOnly _returnvalue false)
      (Variables|/Script/Engine.PlayerController|SetbShowMouseCursor (Game|GetPlayerController 0) false))))

(event Game|Damage|EventAnyDamage
  (params (Damage :type Float%20%28single-precision%29) (DamageType :type Damage%20Type%20Object%20Reference) (InstigatedBy :type Controller%20Object%20Reference) (DamageCauser :type Actor%20Object%20Reference))
  (bind _max_health (Variables|Default|Getmax_health))
  ;[0.15 0.15 0.15 0.5] GESTIONE DELL'INTERFACCIA GRAFICA DEL PLAYER
  ;;[0.15 0.15 0.15 0.5] Calcola i danni subiti dal player
  (bind _output_get (Variables|Default|Setcurrent_health (Math|Float|Clamp(Float) (- (Variables|Default|Getcurrent_health) Damage) 0.0 _max_health)))
  (Default|UIUpdateHealth (Variables|Default|GetUI_main) _output_get _max_health))

(event EventRestarted
  (bind _max_health (Variables|Default|Getmax_health))
  ;[0.15 0.15 0.15 0.5] GESTIONE DELL'INTERFACCIA GRAFICA DEL PLAYER
  ;;[0.15 0.15 0.15 0.5] All'avvio del gioco, mostra l'interfaccia grafica del player e imposta al massimo la sua vita attuale
  (bind _returnvalue (UserInterface|CreateWidget "/Game/Interfaccia_Grafica/UI_Player.UI_Player_C" (Game|GetPlayerController 0)))
  (bind _output_get (Variables|Default|SetUI_main _returnvalue))
  (UserInterface|Viewport|AddtoViewport _output_get 0)
  (bind _output_get_2 (Variables|Default|Setcurrent_health _max_health))
  (Default|UIUpdateHealth (Variables|Default|GetUI_main) _output_get_2 _max_health))

(event Input|ActionEvents|InputActionSalto
  (params (Key :type Key%20Structure :default "None"))
  ;[0.15 0.15 0.15 0.5] MOVIMENTO DEL PLAYER
  ;;[0.15 0.15 0.15 0.5] Quando premo la barra spaziatrice, il player salta
  (:Pressed
    (Character|Jump)))

(event Input|ActionEvents|InputActionAvanti
  (params (Key :type Key%20Structure :default "None"))
  ;[0.15 0.15 0.15 0.5] MOVIMENTO DEL PLAYER
  ;;[0.15 0.15 0.15 0.5] Se premo il tasto "D" ruota il player, in modo che punti a destra
  (:Pressed
    (Transformation|SetRelativeRotation (Variables|Character|GetMesh) "0, 0, 0" false false)))

(event Input|ActionEvents|InputActionIndietro
  (params (Key :type Key%20Structure :default "None"))
  ;[0.15 0.15 0.15 0.5] MOVIMENTO DEL PLAYER
  ;;[0.15 0.15 0.15 0.5] Se premo il tasto "A" ruota il player, in modo che punti a sinistra
  (:Pressed
    (Transformation|SetRelativeRotation (Variables|Character|GetMesh) "0.000000,180.000000,0.000000" false false)))

(event Input|AxisEvents|InputAxisAvanti
  (params (AxisValue :type Float%20%28single-precision%29))
  ;[0.15 0.15 0.15 0.5] MOVIMENTO DEL PLAYER
  ;;[0.15 0.15 0.15 0.5] Se premo il tasto "D" il player si muove a destra
  (Pawn|Input|AddMovementInput (Math|Vector|GetForwardVector (Variables|Collision|GetCapsuleComponent)) AxisValue false))

(event Input|AxisEvents|InputAxisIndietro
  (params (AxisValue :type Float%20%28single-precision%29))
  ;[0.15 0.15 0.15 0.5] MOVIMENTO DEL PLAYER
  ;;[0.15 0.15 0.15 0.5] Se premo il tasto "A" il player si muove a sinistra
  (Pawn|Input|AddMovementInput (- "" (Math|Vector|GetForwardVector (Variables|Collision|GetCapsuleComponent))) AxisValue false))

(event Input|KeyboardEvents|E
  (params (Key :type Key%20Structure :default "None"))
  (bind _returnvalue (Transformation|GetActorLocation))
  (bind _mesh (Variables|Character|GetMesh))
  (bind _blocco (Variables|Default|GetBlocco))
  (bind _returnvalue_2 (Math|Vector|GetForwardVector _mesh))
  (bind _returnvalue_3 (* _returnvalue_2 "300.000000,0.000000,0.000000"))
  (bind _returnvalue_4 (+ _returnvalue _returnvalue_3))
  ;[0.15 0.15 0.15 0.5] RACCOLTA BLOCCO
  (:Pressed
    (if (Variables|Default|GetCarrying)
      ;[0.15 0.15 0.15 0.5] POSIZIONA BLOCCO
      (bind _outactors (Collision|BoxOverlapActors _returnvalue_4 "10.000000,10.000000,10.000000" (Utilities|Array|MakeArray "ObjectTypeQuery2") 0 :!class /Script/Engine.KismetSystemLibrary))
      (if (Utilities|Array|IsEmpty _outactors)
        (bind _returnvalue_5 (Game|SpawnActorfromClass "/Game/Blocchi/BP_Blocco_Sollevabile.BP_Blocco_Sollevabile_C" (Math|Transform|MakeTransform _returnvalue_4 (Variables|/Script/Engine.SceneComponent|GetRelativeRotation (Variables|Character|GetMesh)) "1.000000,1.000000,1.000000") "Undefined" "MultiplyWithRoot" 0 0))
        (Components|StaticMesh|SetStaticMesh (Variables|/Game/Blocchi/BP_Blocco_Sollevabile.BP_Blocco_Sollevabile_C|GetBlocco_di_cemento _returnvalue_5) (Variables|/Script/Engine.StaticMeshComponent|GetStaticMesh (Variables|Default|GetBlocco)))
        (Rendering|SetVisibility (Variables|Default|GetBlocco) false false)
        (Variables|Default|SetCarrying false))
      (else
        (bind _array_element (Utilities|Array|ForEachLoopwithBreak (Collision|GetOverlappingActors "/Game/Blocchi/BP_Blocco_Sollevabile.BP_Blocco_Sollevabile_C" :!class /Script/Engine.Actor) :!label _label)
          (:LoopBody
            (if (Utilities|DoesObjectImplementInterface _array_element "/Game/Blocchi/PU_Interface.PU_Interface_C")
              (Class|PUInterface|PickUp(Message) _array_element)
              (bind _asbp_blocco_sollevabile (Utilities|Casting|CastToBP_Blocco_Sollevabile _array_element))
              (Components|StaticMesh|SetStaticMesh _blocco (Variables|/Script/Engine.StaticMeshComponent|GetStaticMesh (Variables|/Game/Blocchi/BP_Blocco_Sollevabile.BP_Blocco_Sollevabile_C|GetBlocco_di_cemento _asbp_blocco_sollevabile)))
              (Rendering|SetVisibility _blocco true false)
              (Variables|Default|SetCarrying true)
              (goto _label Break))))))))

(event Input|KeyboardEvents|Z
  (params (Key :type Key%20Structure :default "None"))
  (bind _returnvalue (Game|GetPlayerController 0))
  ;[0.15 0.15 0.15 0.5] (MENU DI PAUSA) Quando premo "Esc", se il menù di pausa è chiuso, lo apri; ALTRIMENTI, se il menù di pausa è aperto, lo chiudi
  (:Pressed
    (if (not (Variables|Default|Getmenu_pausa_aperto?))
      (Variables|Default|Setmenu_pausa_aperto? true)
      (bind _returnvalue_2 (UserInterface|CreateWidget "/Game/Interfaccia_Grafica/UI_Pause_Menu.UI_Pause_Menu_C" _returnvalue))
      (bind _output_get (Variables|Default|Setui_menu_pausa _returnvalue_2))
      (UserInterface|Viewport|AddtoViewport _output_get 0)
      (Input|SetInputModeGameandUI _returnvalue (Variables|Default|Getui_menu_pausa) "DoNotLock" true false)
      (Variables|/Script/Engine.PlayerController|SetbShowMouseCursor (Game|GetPlayerController 0) true)
      (Game|SetGamePaused true)
      (else
        (Variables|Default|Setmenu_pausa_aperto? false)
        (Widget|RemovefromParent (Variables|Default|Getui_menu_pausa))
        (Game|SetGamePaused false)
        (Input|SetInputModeGameOnly _returnvalue false)
        (Variables|/Script/Engine.PlayerController|SetbShowMouseCursor (Game|GetPlayerController 0) false)))))

(fn ConstructionScript)

(fn CanTakeDMG
  (params (A :type Object%20Object%20Reference) (Object :type Object%20Object%20Reference))
  (bind _asbp_blocco_sollevabile (Utilities|Casting|CastToBP_Blocco_Sollevabile Object)
    (:then
      (if (and (== (Variables|/Game/Blocchi/BP_Blocco_Sollevabile.BP_Blocco_Sollevabile_C|GetDMG_Trigger _asbp_blocco_sollevabile) A) (and (== (Variables|/Game/Blocchi/BP_Blocco_Sollevabile.BP_Blocco_Sollevabile_C|GetMesh _asbp_blocco_sollevabile) "/Game/Modelli_3D/MODELLI_3D_Oggetti/Cono/Cono.Cono") (Variables|/Game/Blocchi/BP_Blocco_Sollevabile.BP_Blocco_Sollevabile_C|GetCanDMG _asbp_blocco_sollevabile)))
        (return _asbp_blocco_sollevabile)))
    (:CastFailed
      (return _asbp_blocco_sollevabile))))